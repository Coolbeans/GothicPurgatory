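; Revolver weapon Blueprint that handles firing and reloading with procedural animation of the gun body, hammer and chamber.
; Fire calls the hitscan, spawns a BP_Projectile at the firing point and runs a recoil timeline rotating the body and hammer before snapping them back.
; Reload moves the chamber out, spins it on a timeline, then restores it.
; A DoOnce limits this animation to one play until Fire resets it.
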(event EventBeginPlay
  (|CallParentFunction)
  (Variables|Default|SetGunStartLoc (Variables|/Script/Engine.SceneComponent|GetRelativeRotation (Variables|Default|GetGun_Body))))

(event EventReload
  (Utilities|FlowControl|DoOnce false
    (:Completed
      (Transformation|SetRelativeLocation (Variables|Default|GetGun_Chamber) (Variables|Default|GetChamberEndLoc) false false)
      (bind _newtrack_0 (Timeline|ChamberLerp PlayFromStart)
        (:Update
          (Transformation|SetRelativeRotation (Variables|Default|GetGun_Chamber) (Math|Rotator|Lerp(Rotator) (Variables|Default|GetChamberStartRot) (Variables|Default|GetChamberEndRot) _newtrack_0 true) false false))
        (:Finished
          (Transformation|SetRelativeLocation (Variables|Default|GetGun_Chamber) (Variables|Default|GetChamberStartLoc) false false)
          (Transformation|SetRelativeRotation (Variables|Default|GetGun_Chamber) (Variables|Default|GetChamberStartRot) false false))))))

(event EventFire
  (Utilities|FlowControl|Sequence
    (:then_0
      (CallFunction|FireHitScan)
      (Game|SpawnActorfromClass "/Game/Blueprints/Weapons/BP_Projectile.BP_Projectile_C" (Transformation|GetWorldTransform (Variables|Default|GetFiringPoint)) "Undefined" "MultiplyWithRoot" 0 0)
      (bind _lerp (Timeline|GunShootLerp PlayFromStart)
        (:Update
          (Transformation|SetRelativeRotation (Variables|Default|GetGun_Body) (Math|Rotator|Lerp(Rotator) (Variables|Default|GetGunStartLoc) (Variables|Default|GetGunEndLoc) _lerp true) false false)
          (Transformation|SetRelativeRotation (Variables|Default|GetGun_Hammer) (Math|Rotator|Lerp(Rotator) (Variables|Default|GetHammerStartRot) (Variables|Default|GetHammerEndRot) _lerp true) false false))
        (:Finished
          (Transformation|SetRelativeRotation (Variables|Default|GetGun_Body) (Variables|Default|GetGunStartLoc) false false)
          (Transformation|SetRelativeRotation (Variables|Default|GetGun_Hammer) (Variables|Default|GetHammerStartRot) false false))))
    (:then_1
      (Utilities|FlowControl|DoOnce false) ; enters at Reset
    )))

(fn ConstructionScript
  (|CallParentFunction))