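; Base weapon Blueprint that caches its parent actor as the owning third-person character on BeginPlay.
; Equip, Stow, Fire and Reload are empty events, with hitscan logic in a separate FireHitScan function.
; FireHitScan traces from the follow camera out to Range, stores that hit, then traces from FiringPoint to it with debug drawing.
; The second trace's result is unused and marked for change, spread is unconnected, and no damage is applied.
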(event Custom|Reload)

(event Custom|Equip)

(event Custom|Stow)

(event Custom|Fire)

(event EventBeginPlay
  (bind _asbp_third_person_character (Utilities|Casting|CastToBP_ThirdPersonCharacter (Actor|GetParentActor)))
  (Variables|Default|SetPlayerRef _asbp_third_person_character))

(fn ConstructionScript)

(fn FireHitScan
  (bind _playerref (Variables|Default|GetPlayerRef))
  (bind _followcamera (Variables|/Game/ThirdPerson/Blueprints/BP_ThirdPersonCharacter.BP_ThirdPersonCharacter_C|GetFollowCamera _playerref))
  (bind _returnvalue (Transformation|GetWorldLocation _followcamera))
  (bind _outhit (Collision|LineTraceByChannel _returnvalue (+ _returnvalue (* (Math|Vector|GetForwardVector _followcamera) (Variables|Default|GetRange))) "TraceTypeQuery1" false (Utilities|Array|MakeArray (Variables|Default|GetPlayerRef) self) "None" true "(R=0.000000,G=0.055354,B=1.000000,A=1.000000)"))
  (Variables|Default|SetHitInfoL _outhit)
  (Collision|LineTraceByChannel (Transformation|GetWorldLocation (Variables|Default|GetFiringPoint)) (.Location (Collision|BreakHitResult _outhit)) "TraceTypeQuery1" false (Utilities|Array|MakeArray (Variables|Default|GetPlayerRef) self) (select (Variables|Default|GetDrawDebug?) "ForDuration" "ForOneFrame")))