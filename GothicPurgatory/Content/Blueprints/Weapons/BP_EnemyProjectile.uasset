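; BP_EnemyProjectile is an enemy projectile that damages the player character.
; It destroys itself after a short delay from BeginPlay.
; When its collision sphere ends an overlap with the player's BP_ThirdPersonCharacter, it applies BulletDamage with itself as the damage causer.
; The damage triggers on overlap end rather than begin, is limited to one hit by a DoOnce, and does not destroy the projectile.
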(event OnComponentEndOverlap(SphereCollision)
  (params (OverlappedComponent :type Primitive%20Component%20Object%20Reference) (OtherActor :type Actor%20Object%20Reference) (OtherComp :type Primitive%20Component%20Object%20Reference) (OtherBodyIndex :type Integer))
  (bind _returnvalue (Game|GetPlayerCharacter 0))
  (bind _asbp_third_person_character (Utilities|Casting|CastToBP_ThirdPersonCharacter _returnvalue))
  (if (== OtherActor _asbp_third_person_character)
    (Utilities|FlowControl|DoOnce false
      (:Completed
        (Game|Damage|ApplyDamage _asbp_third_person_character (Variables|Default|GetBullet%20damage) 0 self)))))

(event EventBeginPlay
  (Utilities|FlowControl|Delay 3.0)
  (Actor|DestroyActor))

(fn ConstructionScript)