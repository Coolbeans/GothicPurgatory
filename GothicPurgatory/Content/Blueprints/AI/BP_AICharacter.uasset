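; AI enemy character that tracks health, shows it on an overhead healthbar widget and dies when it runs out.
; AnyDamage clamps health, and non-lethal hits refresh the healthbar, report a damage event to AI perception and briefly pulse the DeathVFX effect.
; On death it unpossesses the AI controller, ragdolls the mesh, disables capsule collision, hides the healthbar and expires after a short lifespan.
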(event Custom|EnemyDeath
  (bind _self self)
  (bind _mesh (Variables|Character|GetMesh))
  (bind _returnvalue (AI|GetAIController _self))
  (Utilities|IsValid _returnvalue
    (:Is%20Valid
      (Pawn|UnPossess _returnvalue))
    (:Is%20Not%20Valid
      _))
  (Collision|SetCollisionEnabled _mesh "PhysicsOnly")
  (Physics|SetSimulatePhysics _mesh true)
  (Collision|SetCollisionEnabled (Variables|Collision|GetCapsuleComponent) "NoCollision")
  (Actor|SetLifeSpan 3.0)
  (Rendering|SetVisibility (Variables|Default|GetHealthbar) false false))

(event EventBeginPlay
  (Variables|Default|SetCurrentHealth (Variables|Default|GetMaxHealth))
  (bind _aswb_enemy_healthbar (Utilities|Casting|CastToWB_EnemyHealthbar (UserInterface|GetWidget (Variables|Default|GetHealthbar))))
  (Variables|/Game/UI/WB_EnemyHealthbar.WB_EnemyHealthbar_C|SetWBP_CurrentHeatlh _aswb_enemy_healthbar (Variables|Default|GetCurrentHealth))
  (Variables|/Game/UI/WB_EnemyHealthbar.WB_EnemyHealthbar_C|SetWBP_MaxHealth _aswb_enemy_healthbar (Variables|Default|GetMaxHealth)))

(event Game|Damage|EventAnyDamage
  (params (Damage :type Float%20%28single-precision%29) (DamageType :type Damage%20Type%20Object%20Reference) (InstigatedBy :type Controller%20Object%20Reference) (DamageCauser :type Actor%20Object%20Reference))
  (bind _deathvfx (Variables|Default|GetDeathVFX))
  (bind _output_get (Variables|Default|SetCurrentHealth (Math|Float|Clamp(Float) (- (Variables|Default|GetCurrentHealth) Damage) 0.0 (Variables|Default|GetMaxHealth))))
  (if (<= _output_get 0.0)
    (CallFunction|EnemyDeath)
    (else
      (Utilities|FlowControl|Sequence
        (:then_0
          (Class|AISenseDamage|ReportDamageEvent self DamageCauser Damage (Transformation|GetActorLocation) "0, 0, 0" "None")
          (bind _aswb_enemy_healthbar (Utilities|Casting|CastToWB_EnemyHealthbar (UserInterface|GetWidget (Variables|Default|GetHealthbar))))
          (Variables|/Game/UI/WB_EnemyHealthbar.WB_EnemyHealthbar_C|SetWBP_CurrentHeatlh _aswb_enemy_healthbar (Variables|Default|GetCurrentHealth))
          (Variables|/Game/UI/WB_EnemyHealthbar.WB_EnemyHealthbar_C|SetWBP_MaxHealth _aswb_enemy_healthbar (Variables|Default|GetMaxHealth)))
        (:then_1
          (Components|Activation|Activate _deathvfx false)
          (Utilities|FlowControl|Delay 0.1)
          (Components|Activation|Deactivate _deathvfx))))))

(fn ConstructionScript)