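; BP_MySaveData is a save data object that stores and restores the player's quest state.
; SaveQuestLog copies the active and completed quest lists, while SaveQuestDetails records each quest's stage and objective progress in a map keyed by quest ID.
; LoadQuests re-adds every active quest through the quest log component, applies its saved stage and progress, then overwrites the component's two lists with the saved ones.
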(fn SaveQuestDetails
  (params (Quest :type BP%20Quest%20Base%20Object%20Reference))
  (Utilities|Map|Add (Variables|Default|GetQuestProgress) (Variables|/Game/Blueprints/QuestSystem/BP_Quest_Base.BP_Quest_Base_C|GetQuestID Quest) (Utilities|Struct|MakeST_FQuestSaveData (Variables|/Game/Blueprints/QuestSystem/BP_Quest_Base.BP_Quest_Base_C|GetCurrentObjectiveProgress Quest) (Variables|/Game/Blueprints/QuestSystem/BP_Quest_Base.BP_Quest_Base_C|GetCurrentStage Quest))))

(fn LoadQuests
  (params (QuestLogComponent :type BP%20Quest%20Log%20Component%20Object%20Reference))
  (for _array_element (Variables|Default|GetCurrentActiveQuests)
    (bind _returnvalue (Default|AddNewQuest QuestLogComponent _array_element))
    (Variables|/Game/Blueprints/QuestSystem/BP_Quest_Base.BP_Quest_Base_C|SetCurrentStage _returnvalue (.CurrentStage (Utilities|Struct|BreakST_FQuestSaveData (.Value (Utilities|Map|Find (Variables|Default|GetQuestProgress) _array_element)))))
    (Variables|/Game/Blueprints/QuestSystem/BP_Quest_Base.BP_Quest_Base_C|SetCurrentObjectiveProgress _returnvalue (.Progress (Utilities|Struct|BreakST_FQuestSaveData (.Value (Utilities|Map|Find (Variables|Default|GetQuestProgress) _array_element))))))
  (Variables|/Game/Blueprints/QuestSystem/BP_QuestLogComponent.BP_QuestLogComponent_C|SetCurrentActiveQuests QuestLogComponent (Variables|Default|GetCurrentActiveQuests))
  (Variables|/Game/Blueprints/QuestSystem/BP_QuestLogComponent.BP_QuestLogComponent_C|SetCompletedQuests QuestLogComponent (Variables|Default|GetCompletedQuests)))

(fn SaveQuestLog
  (params (QuestLog :type BP%20Quest%20Log%20Component%20Object%20Reference))
  (Variables|Default|SetCurrentActiveQuests (Variables|/Game/Blueprints/QuestSystem/BP_QuestLogComponent.BP_QuestLogComponent_C|GetCurrentActiveQuests QuestLog))
  (Variables|Default|SetCompletedQuests (Variables|/Game/Blueprints/QuestSystem/BP_QuestLogComponent.BP_QuestLogComponent_C|GetCompletedQuests QuestLog)))