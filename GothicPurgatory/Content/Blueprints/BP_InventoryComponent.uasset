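; BP_InventoryComponent is an inventory component that tracks item quantities in a Content map.
; AddToInventory adds the quantity to the stored count, then casts player character 0 to BP_ThirdPersonCharacter and calls its objective notification with the item as ID and the added amount as value.
; QueryInventory returns the stored count for an item.
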(event EventBeginPlay)

(event EventTick
  (params (DeltaSeconds :type Float%20%28single-precision%29)))

(fn AddtoInventory
  (params (Item :type Name) (Quantity :type Integer))
  (Utilities|Map|Add (Variables|Default|GetContent) Item (+ Quantity (.Value (Utilities|Map|Find (Variables|Default|GetContent) Item))))
  (bind _asbp_third_person_character (Utilities|Casting|CastToBP_ThirdPersonCharacter (Game|GetPlayerCharacter 0)))
  (Default|CallOnObjectiveIDCalled _asbp_third_person_character (Utilities|String|ToString(Name) Item) Quantity))

(fn QueryInventory
  (params (Item :type Name))
  (return (.Value (Utilities|Map|Find (Variables|Default|GetContent) Item))))