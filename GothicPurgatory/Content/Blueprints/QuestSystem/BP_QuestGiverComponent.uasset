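; Quest giver component that lets its owning actor offer a quest, referenced by a data table row handle, through an Interaction function.
; Interaction asks the player character's quest log component whether that quest is already active.
; If not, DisplayQuest looks up the row and prints the quest name; otherwise it prints an already-on-quest message.
; Both branches return the owner's display name, and output is only debug prints.
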(event EventBeginPlay)

(event EventTick
  (params (DeltaSeconds :type Float%20%28single-precision%29)))

(fn DisplayQuest
  (bind _questdata (Variables|Default|GetQuestData))
  (bind _returnvalue (Utilities|GetDataTableRow (.datatable _questdata) (.rowname _questdata))
    (:then
      (Development|PrintString (Utilities|String|ToString(Text) (.QuestName (Utilities|Struct|BreakST_FQuestDetails _returnvalue)))))))

(fn Interaction
  (params (Instigator :type Actor%20Object%20Reference))
  (bind _returnvalue (Components|GetOwner))
  (bind _returnvalue_2 (Utilities|GetDisplayName _returnvalue))
  (if (not (Default|QueryActiveQuest (Variables|/Game/ThirdPerson/Blueprints/BP_ThirdPersonCharacter.BP_ThirdPersonCharacter_C|GetBP_QuestLogComponent (CallFunction|GetMyPlayerCharacter)) (.rowname (Variables|Default|GetQuestData))))
    (CallFunction|DisplayQuest)
    (return _returnvalue_2)
    (else
      (Development|PrintString "Already on quest")
      (return _returnvalue_2))))