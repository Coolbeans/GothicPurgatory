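; Base quest Blueprint that tracks objective progress for the current stage of a quest loaded from DT_QuestData by QuestID.
; On BeginPlay it fills a progress map, binds to the player character's objective-ID event and seeds one objective type from inventory counts.
; Heard IDs adjust progress, including decreases for lost quest items.
; Reaching an objective's quantity shows a notification widget and re-evaluates IsCompleted across the stage.
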(event EventBeginPlay
  (CallFunction|GetQuestDetails)
  (EventDispatchers|BindEventtoOnObjectiveIDCalled (CallFunction|GetMyPlayerCharacter) (EventDispatchers|CreateEvent :!event OnObjectiveIDHeard))
  (for _array_element (.Objectives (Utilities|Struct|BreakST_FStageDetails (Variables|Default|GetCurrentStageDetails)))
    (if (Utilities|Enum|Equal(Enum) (.Type (Utilities|Struct|BreakST_FObjectiveDetails _array_element)) "NewEnumerator3")
      (bind _value (Default|QueryInventory (Variables|/Game/ThirdPerson/Blueprints/BP_ThirdPersonCharacter.BP_ThirdPersonCharacter_C|GetBP_InventoryComponent (CallFunction|GetMyPlayerCharacter)) (Utilities|String|StringToName (.ObjectiveID (Utilities|Struct|BreakST_FObjectiveDetails _array_element)))))
      (CallFunction|OnObjectiveIDHeard (.ObjectiveID (Utilities|Struct|BreakST_FObjectiveDetails _array_element)) _value)))
  (bind _return (CallFunction|AreObjectivesComplete))
  (Variables|Default|SetIsCompleted? _return))

(fn ConstructionScript)

(fn OnObjectiveIDHeard
  (params (ObjectiveID :type String) (Value :type Integer))
  (bind _currentobjectiveprogress (Variables|Default|GetCurrentObjectiveProgress))
  (bind (_value _returnvalue) (Utilities|Map|Find _currentobjectiveprogress ObjectiveID))
  (if (> (Class|KismetMathLibrary|SignOfInteger Value) 0)
    (if _returnvalue
      (if (< _value (.Quantity (Utilities|Struct|BreakST_FObjectiveDetails (CallFunction|GetObjectiveDatabyID ObjectiveID))))
        (Utilities|Map|Add (Variables|Default|GetCurrentObjectiveProgress) ObjectiveID (+ _value Value))
        (CallFunction|IsObjectiveComplete? ObjectiveID)
        (return))
      (else
        (return)))
    (else
      ;[1 1 1] To update on inventory item loss for quest item
      (Utilities|Map|Add (Variables|Default|GetCurrentObjectiveProgress) ObjectiveID (+ (.Value (Utilities|Map|Find (Variables|Default|GetCurrentObjectiveProgress) ObjectiveID)) Value))
      (return))))

(fn GetQuestDetails
  (bind _returnvalue (Utilities|GetDataTableRow "/Game/Blueprints/QuestSystem/DT_QuestData.DT_QuestData" (Variables|Default|GetQuestID))
    (:then
      (bind _output_get (Variables|Default|SetQuestDetails _returnvalue))
      (bind _output_get_2 (Variables|Default|SetCurrentStageDetails (Utilities|Array|Get(acopy) (.Stages (Utilities|Struct|BreakST_FQuestDetails _output_get)) (Variables|Default|GetCurrentStage))))
      (Utilities|Map|Clear (Variables|Default|GetCurrentObjectiveProgress))
      (for _array_element (.Objectives (Utilities|Struct|BreakST_FStageDetails _output_get_2))
        (Utilities|Map|Add (Variables|Default|GetCurrentObjectiveProgress) (.ObjectiveID (Utilities|Struct|BreakST_FObjectiveDetails _array_element)) 0)))))

(fn GetObjectiveDatabyID
  (params (ObjectiveID :type String))
  (for _array_element (.Objectives (Utilities|Struct|BreakST_FStageDetails (Variables|Default|GetCurrentStageDetails)))
    (if (Utilities|Enum|Equal(Enum) ObjectiveID (.ObjectiveID (Utilities|Struct|BreakST_FObjectiveDetails _array_element)))
      (return _array_element))))

(fn IsObjectiveComplete?
  (params (ObjectiveID :type String))
  (bind _array_element (CallFunction|GetObjectiveDatabyID ObjectiveID))
  (bind (_objectivename _description _type _objectiveid _quantity) (Utilities|Struct|BreakST_FObjectiveDetails _array_element))
  (if (>= (.Value (Utilities|Map|Find (Variables|Default|GetCurrentObjectiveProgress) ObjectiveID)) _quantity)
    (bind _returnvalue (UserInterface|CreateWidget "/Game/UI/QuestWidgets/WBP_QuestNotification.WBP_QuestNotification_C" 0 _description))
    (UserInterface|Viewport|AddtoViewport _returnvalue 0)
    (bind _return (CallFunction|AreObjectivesComplete))
    (Variables|Default|SetIsCompleted? _return)))

(fn AreObjectivesComplete
  (for _array_element (.Objectives (Utilities|Struct|BreakST_FStageDetails (Variables|Default|GetCurrentStageDetails)))
    (if (not (>= (.Value (Utilities|Map|Find (Variables|Default|GetCurrentObjectiveProgress) (.ObjectiveID (Utilities|Struct|BreakST_FObjectiveDetails _array_element)))) (.Quantity (Utilities|Struct|BreakST_FObjectiveDetails (CallFunction|GetObjectiveDatabyID (.ObjectiveID (Utilities|Struct|BreakST_FObjectiveDetails _array_element)))))))
      (bind _output_get (LocalVariables|SetLocal_AllComplete false))
      (return _output_get)))
  (return (LocalVariables|GetLocal_AllComplete)))