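; Quest log component that records active and completed quests by ID and handles adding, tracking and turn-in.
; Each new quest spawns a BP_Quest_Base actor, which is looked up by ID for completion and status queries.
; Turn-in only prints the stage's XP reward, then completes the quest, flagging the actor and firing OnQuestCompleted.
; Tracking creates one WBP_QuestTracker widget on first use and updates it afterwards.
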(event EventBeginPlay)

(event EventTick
  (params (DeltaSeconds :type Float%20%28single-precision%29)))

(fn AddNewQuest
  (params (QuestID :type Name))
  (Utilities|Array|AddUnique (Variables|Default|GetCurrentActiveQuests) QuestID)
  (bind _returnvalue (Game|SpawnActorfromClass "/Game/Blueprints/QuestSystem/BP_Quest_Base.BP_Quest_Base_C" (Math|Transform|MakeTransform "0, 0, 0" "0, 0, 0" "1.000000,1.000000,1.000000") "Undefined" "MultiplyWithRoot" 0 QuestID 0))
  (Utilities|Array|Add (Variables|Default|GetCurrentQuests) _returnvalue)
  (return _returnvalue))

(fn CompleteQuest
  (params (QuestID :type Name))
  (Utilities|Array|AddUnique (Variables|Default|GetCompletedQuests) QuestID)
  (Utilities|Array|RemoveItem (Variables|Default|GetCurrentActiveQuests) QuestID)
  (bind _array_element (CallFunction|GetQuestActor QuestID))
  (Variables|/Game/Blueprints/QuestSystem/BP_Quest_Base.BP_Quest_Base_C|SetIsTurnedIn? _array_element true)
  (Default|CallOnQuestCompleted _array_element))

(fn QueryActiveQuest
  (params (QuestID :type Name))
  (return (Utilities|Array|ContainsItem (Variables|Default|GetCurrentActiveQuests) QuestID)))

(fn TrackQuest
  (params (QuestActor :type BP%20Quest%20Base%20Object%20Reference))
  (bind _trackerwidget (Variables|Default|GetTrackerWidget)
    (:then
      (Default|Update _trackerwidget QuestActor))
    (:else
      (bind _returnvalue (UserInterface|CreateWidget "/Game/UI/QuestWidgets/WBP_QuestTracker.WBP_QuestTracker_C" 0 QuestActor))
      (bind _output_get (Variables|Default|SetTrackerWidget _returnvalue))
      (UserInterface|Viewport|AddtoViewport _output_get -1))))

(fn GetQuestActor
  (params (QuestID :type Name))
  (for _array_element (Variables|Default|GetCurrentQuests)
    (if (== (Variables|/Game/Blueprints/QuestSystem/BP_Quest_Base.BP_Quest_Base_C|GetQuestID _array_element) QuestID)
      (return _array_element))))

(fn TurninQuest
  (params (QuestID :type Name))
  (Utilities|FlowControl|Sequence
    (:then_0
      (bind _array_element (CallFunction|GetQuestActor QuestID))
      (Development|PrintString (Utilities|String|ToString(Text) (Utilities|Text|FormatText "XP = {a}" (.XPReward (Utilities|Struct|BreakST_FStageDetails (Variables|/Game/Blueprints/QuestSystem/BP_Quest_Base.BP_Quest_Base_C|GetCurrentStageDetails _array_element)))))))
    (:then_1
      (CallFunction|CompleteQuest QuestID))))

(fn QueryCompletedQuest
  (params (QuestID :type Name))
  (bind _completedquests (Variables|Default|GetCompletedQuests))
  (bind _returnvalue (Utilities|Array|ContainsItem _completedquests QuestID))
  (bind _array_element (CallFunction|GetQuestActor QuestID))
  (Utilities|IsValid _array_element
    (:Is%20Valid
      (return _returnvalue (Variables|/Game/Blueprints/QuestSystem/BP_Quest_Base.BP_Quest_Base_C|GetIsTurnedIn? _array_element)))
    (:Is%20Not%20Valid
      ;[1 1 1] assumption on quest status
      (return _returnvalue true))))