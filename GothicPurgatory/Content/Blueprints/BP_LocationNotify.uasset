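; BP_LocationNotify is a trigger volume actor that shows a location name notification when the player character enters its box.
; On begin overlap it creates a WBP_LocationNotify widget with its LocationName and adds it to the viewport through a DoOnce gate.
; The gate resets three seconds after the player exits the box, limiting repeat notifications.
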(event OnComponentBeginOverlap(Box)
  (params (OverlappedComponent :type Primitive%20Component%20Object%20Reference) (OtherActor :type Actor%20Object%20Reference) (OtherComp :type Primitive%20Component%20Object%20Reference) (OtherBodyIndex :type Integer) (bFromSweep :type Boolean) (SweepResult :type Hit%20Result%20Structure%20%28by%20ref%29))
  (if (== OtherActor (Game|GetPlayerCharacter 0))
    (bind _returnvalue (UserInterface|CreateWidget "/Game/UI/WBP_LocationNotify.WBP_LocationNotify_C" 0 (Variables|LocationName|GetLocation%20Name)))
    (Variables|Default|SetLocationWidget _returnvalue)
    (if (not (UserInterface|Viewport|IsinViewport (Variables|Default|GetLocationWidget)))
      (Utilities|FlowControl|DoOnce false
        (:Completed
          (UserInterface|Viewport|AddtoViewport (Variables|Default|GetLocationWidget) 0))))))

(event OnComponentEndOverlap(Box)
  (params (OverlappedComponent :type Primitive%20Component%20Object%20Reference) (OtherActor :type Actor%20Object%20Reference) (OtherComp :type Primitive%20Component%20Object%20Reference) (OtherBodyIndex :type Integer))
  (if (== OtherActor (Game|GetPlayerCharacter 0))
    (Utilities|FlowControl|Delay 3.0)
    (Utilities|FlowControl|DoOnce false) ; enters at Reset
  ))

(fn ConstructionScript)