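; Mantling component that lets the player character climb onto ledges in front of it.
; While idle, Tick traces downward ahead of the character, validates ledge height, walkable slope and capsule clearance, then shows or hides the mantle widget.
; The Mantle event switches state so Tick lerps the character to the stored landing point over VaultSpeed seconds, without sweeping.
; The trace ignores only one instance each of three hardcoded actor classes.
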(event Custom|Mantle
  (Variables|Default|SetProgress 0.0)
  (Variables|Default|SetStarting%20Location (Transformation|GetActorLocation (Variables|Private|GetOwningCharacter)))
  (Variables|Private|SetMantleState "NewEnumerator2"))

(event EventBeginPlay
  (Variables|Private|SetOwningCharacter (CallFunction|GetMyPlayerCharacter))
  (bind _returnvalue (UserInterface|CreateWidget "/Game/UI/Mantling/WBP_Mantling.WBP_Mantling_C" (.AsPlayer%20Controller (Utilities|Casting|CastToPlayerController (Pawn|GetController (Variables|Private|GetOwningCharacter))))))
  (Variables|Private|SetMantleWidget _returnvalue))

(event EventTick
  (params (DeltaSeconds :type Float%20%28single-precision%29))
  (Utilities|SwitchMantleState
    (:NotMantling
      (bind (_result _endinglocation) (Public|CanMantle))
      (if _result
        (Variables|Default|SetEnding%20Location _endinglocation)
        (if (not (UserInterface|Viewport|IsinViewport (Variables|Private|GetMantleWidget)))
          (UserInterface|Viewport|AddtoViewport (Variables|Private|GetMantleWidget) 0))
        (elif (UserInterface|Viewport|IsinViewport (Variables|Private|GetMantleWidget))
          (Widget|RemovefromParent (Variables|Private|GetMantleWidget)))))
    (:Mantiling
      (Private|TickMantle DeltaSeconds))))

(fn CanMantle
  (bind _owningcharacter (Variables|Private|GetOwningCharacter))
  (bind _returnvalue (Transformation|GetActorLocation _owningcharacter))
  (bind _returnvalue_2 (Transformation|GetActorForwardVector _owningcharacter))
  (bind _returnvalue_3 (* _returnvalue_2 7e+01))
  (bind _returnvalue_4 (+ _returnvalue _returnvalue_3))
  (if (Utilities|Enum|Equal(Enum) (Variables|Private|GetMantleState) "NewEnumerator0")
    (LocalVariables|SetCapsule%28local%29 (Variables|/Script/Engine.Character|GetCapsuleComponent (Variables|Private|GetOwningCharacter)))
    ;[1 0 0] Need to add more actors or something
    (bind _returnvalue_5 (Actor|GetActorOfClass "/Game/Blueprints/AI/SmartObjects/SO_Chair.SO_Chair_C"))
    (bind _returnvalue_6 (Actor|GetActorOfClass "/Game/Blueprints/QuestSystem/BP_TestItem.BP_TestItem_C"))
    (bind _returnvalue_7 (Actor|GetActorOfClass "/Game/Blueprints/QuestSystem/BP_Quest_Interactable.BP_Quest_Interactable_C"))
    ;[1 1 1] Comment
    (bind (_outhit _returnvalue_8) (Collision|LineTraceByChannel (+ _returnvalue_4 (Math|Vector|MakeVector 0.0 0.0 (Components|Capsule|GetScaledCapsuleHalfHeight (LocalVariables|GetCapsule%28local%29)))) (- _returnvalue_4 (Math|Vector|MakeVector 0.0 0.0 (Components|Capsule|GetScaledCapsuleHalfHeight (LocalVariables|GetCapsule%28local%29)))) "TraceTypeQuery1" false (Utilities|Array|MakeArray (Variables|Private|GetOwningCharacter) _returnvalue_5 _returnvalue_6 _returnvalue_7) "None"))
    (if _returnvalue_8
      (bind (_result _endinglocation) (Private|CanMantletoHit (LocalVariables|GetCapsule%28local%29) _outhit))
      (return _result _endinglocation)
      (else
        (return false "0, 0, 0")))
    (else
      (return false "0, 0, 0"))))

(fn CanMantletoHit
  (params (Capsule :type Capsule%20Component%20Object%20Reference) (Hit :type Hit%20Result%20Structure))
  (bind _z (Math|Vector|BreakVector (.location Hit)))
  (bind _returnvalue (Components|Capsule|GetScaledCapsuleRadius Capsule))
  (bind _z_2 (Math|Vector|BreakVector (.traceend Hit)))
  (bind _returnvalue_2 (- _z _z_2))
  (Utilities|FlowControl|Sequence
    (:then_0
      ;[0.8047 1 0] Make sure the ledge is at appropriate height
      (Development|PrintString (Utilities|String|ToString(Float) _returnvalue_2) true true "(R=0.000000,G=1.000000,B=0.007393,A=1.000000)" 0.0)
      (if (not (Math|Float|InRange(Float) _returnvalue_2 (Variables|Private|Constant|GetMinVaultingHeight) (Variables|Private|Constant|GetMaxVaultingHeight)))
        (return false "0, 0, 0")))
    (:then_1
      ;[1 0 0] If its too steep it cant climb on
      (if (< (.Z (Math|Vector|BreakVector (.normal Hit))) (Class|CharacterMovementComponent|GetWalkableFloorZ (Variables|/Script/Engine.Character|GetCharacterMovement (Variables|Private|GetOwningCharacter))))
        (return false "0, 0, 0")))
    (:then_2
      ;[0 1 0.9531] Make sure there is enough room for character
      (bind _output_get (LocalVariables|SetEndingLocation%28Local%29 (+ (.location Hit) (Math|Vector|MakeVector 0.0 0.0 (Components|Capsule|GetScaledCapsuleHalfHeight Capsule)))))
      ;;[1 1 1] Debug disabled
      (bind _result (Private|CheckCapsuleCollision (+ _output_get (Math|Vector|MakeVector 0.0 0.0 _returnvalue)) (Components|Capsule|GetScaledCapsuleHalfHeight Capsule) _returnvalue false))
      (if _result
        (return false "0, 0, 0")))
    (:then_3
      (return true (LocalVariables|GetEndingLocation%28local%29)))))

(fn CheckCapsuleCollision
  (params (Center :type Vector) (HalfHeight :type Float%20%28double-precision%29) (Radius :type Float%20%28double-precision%29) (DrawDebug? :type Boolean))
  (Utilities|FlowControl|Sequence
    (:then_0
      (if DrawDebug?
        (Rendering|Debug|DrawDebugCapsule Center HalfHeight Radius "0, 0, 0" "(R=1.000000,G=0.858323,B=0.000000,A=1.000000)" 0.0 3.0)))
    (:then_1
      (bind _returnvalue (Collision|CapsuleOverlapActors Center Radius HalfHeight (Utilities|Array|MakeArray "ObjectTypeQuery1" "ObjectTypeQuery2" "ObjectTypeQuery4" "ObjectTypeQuery5" "ObjectTypeQuery6") "/Script/Engine.Actor" (Utilities|Array|MakeArray (Variables|Private|GetOwningCharacter))))
      (return _returnvalue))))

(fn TickMantle
  (params (DeltaSeconds :type Float%20%28double-precision%29))
  (Utilities|FlowControl|Sequence
    (:then_0
      (Variables|Default|SetProgress (Math|Float|Clamp(Float) (+ (Variables|Default|GetProgress) (/ DeltaSeconds (Variables|Private|Constant|GetVaultSpeed)))))
      (Transformation|SetActorLocation (Variables|Private|GetOwningCharacter) (Math|Vector|Lerp(Vector) (Variables|Default|GetStarting%20Location) (Variables|Default|GetEnding%20Location) (Variables|Default|GetProgress)) false true))
    (:then_1
      (if (>= (Variables|Default|GetProgress) 1.0)
        (Variables|Private|SetMantleState "NewEnumerator0")))))